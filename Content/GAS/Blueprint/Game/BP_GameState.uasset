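; Game state for a card battle game that drives its flow through the Gameplay Ability System.
; On BeginPlay it grants the listed abilities to its own ability system component, then activates those matching the flow start tag.
; Helpers resolve the current player ID from an index map and find another player's state.
; The opposing monster lookup checks only the first child actor of that player's battle card.
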(event EventBeginPlay
  (bind _pggamestateasc (Variables|Default|GetPGGameStateASC))
  (for _array_element (Variables|GAS|GetActivatableAbilities)
    (GameplayAbilities|GiveAbility _pggamestateasc _array_element 0 -1))
  (Abilities|TryActivateAbilitiesbyTag _pggamestateasc (GameplayTags|MakeGameplayTagContainerfromTag (Variables|GAS|GetFlowStartTag)) true))

(event EventTick
  (params (DeltaSeconds :type Float%20%28single-precision%29)))

(fn ConstructionScript)

(fn GetCurrentPlayerID
  (bind _playeridmap (Variables|Default|GetPlayerIDMap))
  (bind _currentplayerindex (Variables|Default|GetCurrentPlayerIndex))
  (bind (_value _returnvalue) (Utilities|Map|Find _playeridmap _currentplayerindex))
  (if _returnvalue
    (return _value)
    (else
      (return -1))))

(fn GetOtherBattleMonster
  (params (Player :type Player%20State%20Object%20Reference))
  (bind _otherplayer (CallFunction|GetOtherPlayerState Player))
  (bind _returnvalue (Class|PGPlayerState|GetBattleCard _otherplayer))
  (for _array_element (Actor|GetAllChildActors _returnvalue true)
    (bind _aspgmonster (Utilities|Casting|CastToPGMonster _array_element)
      (:then
        (return _aspgmonster))
      (:CastFailed
        (return 0)))))

(fn GetOtherPlayerState
  (params (Player :type Player%20State%20Object%20Reference))
  (for _array_element (Variables|Default|GetPlayerArray)
    (if (!= _array_element Player)
      (bind _aspgplayer_state (Utilities|Casting|CastToPGPlayerState _array_element))
      (return _aspgplayer_state)))
  (return 0))