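; Game state Blueprint in a GAS test folder that starts the game flow through gameplay abilities and tracks the current player.
; On BeginPlay it grants every class in ActivatableAbilities to its own ability system component, then activates abilities matching FlowStartTag.
; GetCurrentPlayerID looks up CurrentPlayerIndex in PlayerIDMap and returns -1 when no entry exists.
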(event EventBeginPlay
  (bind _pggamestateasc (Variables|Default|GetPGGameStateASC))
  (for _array_element (Variables|GAS|GetActivatableAbilities)
    (GameplayAbilities|GiveAbility _pggamestateasc _array_element 0 -1))
  (Abilities|TryActivateAbilitiesbyTag _pggamestateasc (GameplayTags|MakeGameplayTagContainerfromTag (Variables|GAS|GetFlowStartTag)) true))

(event EventTick
  (params (DeltaSeconds :type Float%20%28single-precision%29)))

(fn ConstructionScript)

(fn GetCurrentPlayerID
  (bind _playeridmap (Variables|Default|GetPlayerIDMap))
  (bind _currentplayerindex (Variables|Default|GetCurrentPlayerIndex))
  (bind (_value _returnvalue) (Utilities|Map|Find _playeridmap _currentplayerindex))
  (if _returnvalue
    (return _value)
    (else
      (return -1))))