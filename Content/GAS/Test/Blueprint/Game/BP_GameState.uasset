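; Game state Blueprint that drives game flow through gameplay abilities on its FlowASC component, starting with a wait for deck selection.
; On BeginPlay it grants every class in StartAbilities, then activates abilities tagged Game.Action.WaitSelectedDeck.
; The OnSetGameplayTag event ends the ability matching the received tag, so flow steps are closed by tag rather than by direct reference.
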(event Custom|OnSetGameplayTag
  (params (Gameplay%20Tag :type Gameplay%20Tag%20Structure))
  (Class|PGFlowAbilitySystemComponent|EndAbilitywithTag (Variables|Default|GetFlowASC) (GameplayTags|MakeGameplayTagContainerfromTag Gameplay%20Tag)))

(event EventBeginPlay
  (for _array_element (Variables|Default|GetStartAbilities)
    (GameplayAbilities|GiveAbility (Variables|Default|GetFlowASC) _array_element 0 -1))
  (Abilities|TryActivateAbilitiesbyTag (Variables|Default|GetFlowASC) (GameplayTags|MakeGameplayTagContainerfromTag "(TagName=\"Game.Action.WaitSelectedDeck\")") true))

(event EventTick
  (params (DeltaSeconds :type Float%20%28single-precision%29)))

(fn ConstructionScript)