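; BP_Pawn is a player pawn in a GAS test area that sets up the player's HUD and offers a debug trigger for game readiness.
; On possession by BP_PlayerController, it creates WBP_PlayerFrame, stores it on the controller and adds it to the player screen.
; The TestKey input sends the GameReady gameplay tag to BP_GameState.
; Logic granting StartAbilities through the PlayerState's ASC is present but disconnected, so it never runs.
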(event EventBeginPlay)

(event Collision|EventActorBeginOverlap
  (params (OtherActor :type Actor%20Object%20Reference)))

(event EventTick
  (params (DeltaSeconds :type Float%20%28single-precision%29)))

(event EventPossessed
  (params (NewController :type Controller%20Object%20Reference))
  (bind _asbp_player_controller (Utilities|Casting|CastToBP_PlayerController NewController))
  (bind _returnvalue (UserInterface|CreateWidget "/Game/GAS/UI/WBP_PlayerFrame.WBP_PlayerFrame_C" _asbp_player_controller))
  (bind _output_get (Variables|/Game/GAS/Test/Blueprint/Player/BP_PlayerController.BP_PlayerController_C|SetCurrent%20Widget _asbp_player_controller _returnvalue))
  (UserInterface|Viewport|AddtoPlayerScreen _output_get))

(event Input|ActionEvents|InputActionTestKey
  (params (Key :type Key%20Structure :default "None"))
  (:Pressed
    (bind _asbp_game_state (Utilities|Casting|CastToBP_GameState (Game|GetGameState)))
    (Default|OnSetGameplayTag _asbp_game_state "(TagName=\"Game.Action.GameReady\")")))

(fn ConstructionScript)